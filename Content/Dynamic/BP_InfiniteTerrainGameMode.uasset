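; Game mode for an infinite terrain game that spawns chained BP_Tile actors and keeps a score of tiles conquered.
; On BeginPlay it populates a pool of nav mesh bounds volumes, then spawns an initial run of tiles.
; SpawnTile hands each new tile that shared pool and takes its attach location as the next spawn transform.
; NewTileConquered increments and prints the score, which GetScore exposes.
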(event `self.ReceiveBeginPlay`
  (`self.PopulateBoundsVolumePool`)
  (for _ (range 3)
    (`self.SpawnTile`)))

(fn `GetScore`
  (returns (Score :type Integer))
  (return (`self.Score`)))

(fn `NewTileConquered`
  (bind _result (`/Engine/EditorBlueprintResources/StandardMacros.IncrementInt` (`self.Score`))
    (:`  `
      (`KismetSystemLibrary.PrintString` (`KismetStringLibrary.Concat_StrStr` "Tiles conquered: " (`KismetStringLibrary.Conv_IntToString` _result)) true true (struct :`G` 0.66 :`B` 1.0 :`A` 1.0) 10.0))))

(fn `SpawnTile`
  (bind _returnvalue (`|SpawnActorFromClass` "/Game/Dynamic/Terrain/BP_Tile.BP_Tile_C" (`self.nextTileTransform`) "Undefined" "OverrideRootScale" null null))
  (`Tile.SetPool` _returnvalue (`self.NavMeshBoundVolumePool`))
  (bind _attachtransform (`/Game/Dynamic/Terrain/BP_Tile.GetAttachLocation` _returnvalue))
  (set `self.nextTileTransform` _attachtransform))

(fn `UserConstructionScript`)