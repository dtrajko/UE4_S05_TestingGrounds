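; Infinite-terrain tile that fills itself with props, trees, first aid and enemies on BeginPlay, with enemy counts growing with the game mode's score.
; Its barrier unlocks and turns green while the player overlaps LockingVolume, and the first entry reports the tile conquered.
; When the player enters DestroyVolume, it asks the game mode for a new tile, then destroys itself and attached actors.
; The Arrow component provides the attach transform.
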(event `self.ReceiveBeginPlay`
  (`self.Lock`)
  (`self.PlaceRocks`)
  (`self.Place First Aid`)
  (`self.PlaceTrees`)
  (`self.PlaceActors` "/Game/Dynamic/Terrain/Props/BP_Container.BP_Container_C" 1 3)
  (`self.PlaceActors` "/Game/Dynamic/Terrain/Props/BP_Cart_01.BP_Cart_01_C" 1 2 100.0)
  (`self.PlaceActors` "/Game/Dynamic/Terrain/Props/BP_Fence_02.BP_Fence_02_C" 2 4 100.0)
  (`self.PlaceActors` "/Game/Dynamic/Terrain/Props/BP_Box.BP_Box_C" 2 4 200.0 1.0 2.0)
  (`self.PlaceActors` "/Game/Dynamic/Terrain/Props/BP_SandBags.BP_SandBags_C" 1 2 200.0 1.0 2.0)
  (`self.PlaceActors` "/Game/Dynamic/Terrain/Props/BP_Canister.BP_Canister_C" 4 6 50.0)
  (`self.SpawnEnemies`))

(event `self.LockingVolume.OnComponentBeginOverlap`
  (params (OverlappedComponent :type "PrimitiveComponent Object Reference") (OtherActor :type "Actor Object Reference") (OtherComp :type "PrimitiveComponent Object Reference") (OtherBodyIndex :type Integer) (bFromSweep :type Boolean) (SweepResult :type "HitResult Structure (by ref)"))
  (`self.IsPlayerActor` OtherActor
    (:`then`
      (`self.Unlock`)
      (`self.TileConquered`))))

(event `self.LockingVolume.OnComponentEndOverlap`
  (params (OverlappedComponent :type "PrimitiveComponent Object Reference") (OtherActor :type "Actor Object Reference") (OtherComp :type "PrimitiveComponent Object Reference") (OtherBodyIndex :type Integer))
  (`self.IsPlayerActor` OtherActor
    (:`then`
      (`self.Lock`))))

(event `self.DestroyVolume.OnComponentBeginOverlap`
  (params (OverlappedComponent :type "PrimitiveComponent Object Reference") (OtherActor :type "Actor Object Reference") (OtherComp :type "PrimitiveComponent Object Reference") (OtherBodyIndex :type Integer) (bFromSweep :type Boolean) (SweepResult :type "HitResult Structure (by ref)"))
  (`self.IsPlayerActor` OtherActor
    (:`then`
      (bind _asbp_infinite_terrain_game_mode (cast `/Game/Dynamic/BP_InfiniteTerrainGameMode` (`GameplayStatics.GetGameMode`)))
      (`/Game/Dynamic/BP_InfiniteTerrainGameMode.SpawnTile` _asbp_infinite_terrain_game_mode)
      (bind (_arrayindex _arrayelement) (`/Engine/EditorBlueprintResources/StandardMacros.ReverseForEachLoop` (`self.GetAttachedActors`))
        (:`LoopBody`
          (`self.K2_DestroyActor` _arrayelement))
        (:`Completed`
          (`self.K2_DestroyActor`))))))

(fn `GetAttachLocation`
  (returns (AttachTransform :type "Transform Structure"))
  (return (`SceneComponent.K2_GetComponentToWorld` (`self.Arrow`))))

(fn `Lock`
  (`PrimitiveComponent.SetCollisionEnabled` (`self.Barrier`) "QueryAndPhysics")
  (`PrimitiveComponent.SetMaterial` (`self.Barrier`) 0 "/Game/Dynamic/Terrain/MI_Barrier_Red.MI_Barrier_Red"))

(fn `Place First Aid`
  (`self.PlaceActors` "/Game/Dynamic/Terrain/Props/BP_FirstAid.BP_FirstAid_C" 1 2 100.0 0.5 0.5))

(fn `PlaceRocks`
  (`self.PlaceActors` "/Game/Dynamic/Terrain/Props/BP_Rock1.BP_Rock1_C" 2 4 250.0 0.5 3.0)
  (`self.PlaceActors` "/Game/Dynamic/Terrain/Props/BP_Rock2.BP_Rock2_C" 2 4 250.0 0.5 3.0)
  (`self.PlaceActors` "/Game/Dynamic/Terrain/Props/BP_Rock3.BP_Rock3_C" 2 4 250.0 0.5 3.0))

(fn `PlaceTrees`
  (`self.PlaceActors` "/Game/Dynamic/Terrain/Props/BP_WM_AppleTree.BP_WM_AppleTree_C" 1 2 200.0 0.4 0.6)
  (`self.PlaceActors` "/Game/Dynamic/Terrain/Props/BP_WM_Tree_Birch.BP_WM_Tree_Birch_C" 1 2 200.0 0.4 0.6)
  (`self.PlaceActors` "/Game/Dynamic/Terrain/Props/BP_WM_Tree_Pine.BP_WM_Tree_Pine_C" 4 6 200.0 0.4 0.6))

(fn `SpawnEnemies`
  (bind _asbp_infinite_terrain_game_mode (cast `/Game/Dynamic/BP_InfiniteTerrainGameMode` (`GameplayStatics.GetGameMode`)))
  (bind _score (`/Game/Dynamic/BP_InfiniteTerrainGameMode.GetScore` _asbp_infinite_terrain_game_mode))
  (`self.PlaceAIPawns` "/Game/Dynamic/Character/Behavior/BP_Character.BP_Character_C" (+ (`self.MinEnemies`) _score) (+ _score (`self.MaxEnemies`))))

(fn `TileConquered`
  (locals (IsTileConquered :type Boolean))
  (if (not (`self.IsTileConquered2`))
    (bind _asbp_infinite_terrain_game_mode (cast `/Game/Dynamic/BP_InfiniteTerrainGameMode` (`GameplayStatics.GetGameMode`)))
    (`/Game/Dynamic/BP_InfiniteTerrainGameMode.NewTileConquered` _asbp_infinite_terrain_game_mode)
    (set `self.IsTileConquered2` true)))

(fn `Unlock`
  (`PrimitiveComponent.SetCollisionEnabled` (`self.Barrier`) "NoCollision")
  (`PrimitiveComponent.SetMaterial` (`self.Barrier`) 0 "/Game/Dynamic/Terrain/MI_Barrier_Green.MI_Barrier_Green"))

(fn `UserConstructionScript`)